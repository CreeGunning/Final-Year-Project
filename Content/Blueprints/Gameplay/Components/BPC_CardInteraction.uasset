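; Player controller component for mouse-driven card hovering, grabbing and placement on the desk.
; Each tick the local player traces under the cursor to highlight cards, or smoothly drags the held card within desk bounds.
; Server events handle grab, timed location updates, release, attachment and clicks on ungrabbable cards.
; Drops trace downward for a compatible team slot, with spirit cost and enchantment limits checked client-side before the server deducts them.
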(event `self.ReceiveBeginPlay`
  ;[1 1 1] Init
  (bind _aspc_gameplay (cast `/Game/Blueprints/Gameplay/GameMode/PC_Gameplay` (`self.GetOwner`)))
  (set `self.OwnerPC` _aspc_gameplay)
  (bind _playerstate (`/Game/Blueprints/Gameplay/GameMode/PC_Gameplay.GetPlayerState` _aspc_gameplay))
  (`/Engine/EditorBlueprintResources/StandardMacros.IsValid` _playerstate :!label _label
    (:`Is Valid`
      (set `self.IsLocal` (`Controller.IsLocalPlayerController` _aspc_gameplay))
      (set `self.OwnerPS` _playerstate)
      (if (`self.IsLocal`)
        (bind _returnvalue (`GameplayStatics.GetActorOfClass` "/Game/Blueprints/Gameplay/Desk/bP_Desk.bP_Desk_C"))
        (set `self.Desk` _returnvalue)))
    (:`Is Not Valid`
      (`KismetSystemLibrary.Delay` 0.1)
      (goto _label))))

(event `self.ReceiveTick`
  (params (DeltaSeconds :type "Float (single-precision)"))
  ;[1 1 1] Event tick
  (if (`self.IsLocal`)
    (`|ExecutionSequence`
      (:`then_0`
        (if (`self.IsGrabbingCard`)
          (bind _hoveredcard (`self.HoveredCard` :!label _label_2)
            (:`then`
              (`self.ToggleCardHighlight` _hoveredcard)
              (set `self.HoveredCard` null)
              (`/Game/Blueprints/Gameplay/GameMode/HUD_Gameplay.ToggleHover` (`self.GetHUD`) false null))
            (:`else`))
          (else
            (bind _actor (`self.GetActorUnderMouse`))
            (bind _asbp_master_card (cast `/Game/Blueprints/Gameplay/Card/BP_MasterCard` _actor)
              (:`then`
                (bind _hoveredcard_2 (`self.HoveredCard`)
                  (:`then`
                    (if (!= _asbp_master_card _hoveredcard_2)
                      (`self.ToggleCardHighlight` _hoveredcard_2)
                      (bind _output_get (set `self.HoveredCard` _asbp_master_card :!label _label_3))
                      (`self.ToggleCardHighlight` _output_get true)
                      (if (`/Game/Blueprints/Gameplay/Card/BP_MasterCard.CanHover` (`self.HoveredCard`))
                        (`/Game/Blueprints/Gameplay/GameMode/HUD_Gameplay.ToggleHover` (`self.GetHUD`) true (`self.HoveredCard`))
                        (else
                          (`/Game/Blueprints/Gameplay/GameMode/HUD_Gameplay.ToggleHover` (`self.GetHUD`) false null)))))
                  (:`else`
                    (goto _label_3))))
              (:`CastFailed`
                (goto _label_2))))))
      (:`then_1`
        (if (`self.IsGrabbingCard`)
          (bind _grabbedcard (`self.GrabbedCard`)
            (:`then`
              (`Actor.K2_SetActorLocation` _grabbedcard (`KismetMathLibrary.VInterpTo` (`Actor.K2_GetActorLocation` _grabbedcard) (`self.GetCardDragLocation`) (`GameplayStatics.GetWorldDeltaSeconds`) 5.0) false false))
            (:`else`)))))))

(event `ServerToggleInteract`
  (params (Card :type "/Game/Blueprints/Gameplay/Card/BP_MasterCard Object Reference") (StartInteraction :type Boolean) (InitLocation :type "Vector Structure") (TargetLocation :type "Vector Structure"))
  ;[1 1 1] Toggles interaction logic on server
  (if (`self.CanGrabCard` Card)
    (if StartInteraction
      (`Actor.SetActorEnableCollision` Card false)
      (`/Game/Blueprints/Gameplay/Card/BP_MasterCard.ServerOnGrabbed` Card)
      (`/Game/Blueprints/Gameplay/Card/BP_MasterCard.ServerToggleMovement` Card true InitLocation (`self.OwnerPS`))
      (else
        (`Actor.SetActorEnableCollision` Card true)
        (`/Game/Blueprints/Gameplay/Card/BP_MasterCard.ServerToggleMovement` Card false (0.0 0.0 0.0) null)
        (`/Game/Blueprints/Gameplay/Card/BP_MasterCard.ServerReleaseCard` Card InitLocation TargetLocation)))))

(event `ServerUpdateCardLocation`
  (params (Card :type "/Game/Blueprints/Gameplay/Card/BP_MasterCard Object Reference") (Location :type "Vector Structure"))
  ;[1 1 1] Server updates card location and then it replicates to all clients, since the variable is replicated
  (set `/Game/Blueprints/Gameplay/Card/BP_MasterCard.CurrentMovementLocation` Location Card))

(event `ServerAttachCard`
  (params (Card :type "/Game/Blueprints/Gameplay/Card/BP_MasterCard Object Reference") (CardAttachment :type "/Game/Blueprints/Gameplay/Components/BPC_CardAttachment Object Reference") (InitLocation :type "Vector Structure"))
  ;[1 1 1] Server attach card logic
  (`Actor.SetActorEnableCollision` Card true)
  (`/Game/Blueprints/Gameplay/Card/BP_MasterCard.ServerAttachCard` Card CardAttachment InitLocation)
  (`/Game/Blueprints/Gameplay/Card/BP_MasterCard.ServerToggleMovement` Card false (0.0 0.0 0.0) null))

(event `ServerReduceSpirit`
  (params (Amount :type Integer))
  (bind _ownerps (`self.OwnerPS`))
  ;[1 1 1] Calls to reduce spirit for player
  (set `/Game/Blueprints/Gameplay/GameMode/PS_Gameplay.CurrentSpirit` (- (`/Game/Blueprints/Gameplay/GameMode/PS_Gameplay.CurrentSpirit` _ownerps) Amount) _ownerps))

(event `ServerReduceEventCards`
  (bind _ownerps (`self.OwnerPS`))
  ;[1 1 1] Calls to reduce available event cards to play for this turn, by default its 1 but in case you would want that to be > 1, this helps
  (set `/Game/Blueprints/Gameplay/GameMode/PS_Gameplay.RemainingEventCardsToPlace` (- (`/Game/Blueprints/Gameplay/GameMode/PS_Gameplay.RemainingEventCardsToPlace` _ownerps) 1) _ownerps))

(event `ServerCardClick`
  (params (Card :type "/Game/Blueprints/Gameplay/Card/BP_MasterCard Object Reference"))
  ;[1 1 1] Calls clicked card dispatcher on server
  (`self.ServerClickedCard` Card))

(fn `CanGrabCard`
  (params (Card :type "/Game/Blueprints/Gameplay/Card/BP_MasterCard Object Reference"))
  (returns (Success :type Boolean))
  (if (`/Game/Blueprints/Gameplay/Card/BP_MasterCard.CanGrab` (`local.Card`))
    (if (`/Game/Blueprints/Gameplay/Card/BP_MasterCard.TeamOnlyGrab` (`local.Card`))
      (if (== (`/Game/Blueprints/Gameplay/Card/BP_MasterCard.Team` (`local.Card`)) (`self.GetTeam`))
        (return true)
        (else
          (return false)))
      (else
        (return true)))
    (else
      (return false))))

(fn `GetActorUnderMouse`
  (returns (Actor :type "Actor Object Reference"))
  (bind (_worldlocation _worlddirection) (`PlayerController.DeprojectMousePositionToWorld` (`GameplayStatics.GetPlayerController` 0)))
  (bind _outhit (`KismetSystemLibrary.LineTraceSingle` _worldlocation (+ _worldlocation (* _worlddirection 10000.0)) "TraceTypeQuery1"))
  (return (`.HitActor` (`GameplayStatics.BreakHitResult` _outhit))))

(fn `GetCardDragLocation`
  (returns (Location :type "Vector Structure"))
  (bind (_worldlocation _worlddirection) (`PlayerController.DeprojectMousePositionToWorld` (`GameplayStatics.GetPlayerController` 0)))
  (bind (_origin _boxextent) (`KismetSystemLibrary.GetComponentBounds` (`/Game/Blueprints/Gameplay/Desk/bP_Desk.Box` (`self.Desk`))))
  (bind _outhit (`KismetSystemLibrary.LineTraceSingle` _worldlocation (+ _worldlocation (* _worlddirection 10000.0)) "TraceTypeQuery3" false (`|MakeArray` (`self.GrabbedCard`) :!type "Actor Object Reference")))
  (bind (_returnvalue_x _returnvalue_y) (`KismetMathLibrary.BreakVector` (`KismetMathLibrary.Vector_BoundedToBox` (`KismetMathLibrary.SelectVector` (`.Location` (`GameplayStatics.BreakHitResult` _outhit)) (`.TraceEnd` (`GameplayStatics.BreakHitResult` _outhit)) (`GameplayStatics.BreakHitResult` _outhit)) (- _origin _boxextent) (+ _origin _boxextent))))
  (return (`KismetMathLibrary.MakeVector` _returnvalue_x _returnvalue_y 170.0)))

(fn `GetHUD`
  (returns (HUD :type "/Game/Blueprints/Gameplay/GameMode/HUD_Gameplay Object Reference"))
  (bind _ashud_gameplay (cast `/Game/Blueprints/Gameplay/GameMode/HUD_Gameplay` (`PlayerController.GetHUD` (`GameplayStatics.GetPlayerController` 0))))
  (return _ashud_gameplay))

(fn `GetSpirit`
  (returns (Spirit :type Integer))
  (return (`/Game/Blueprints/Gameplay/GameMode/PS_Gameplay.CurrentSpirit` (`self.OwnerPS`))))

(fn `GetTeam`
  (returns (Team :type Integer))
  (return (`/Game/Blueprints/Gameplay/GameMode/PS_Gameplay.Team` (`self.OwnerPS`))))

(fn `IsAttachmentBelow`
  (returns (Success :type Boolean) (AttachmentComp :type "/Game/Blueprints/Gameplay/Components/BPC_CardAttachment Object Reference"))
  (bind _grabbedcard (`self.GrabbedCard`))
  (bind _returnvalue (`Actor.K2_GetActorLocation` (`self.GrabbedCard`)))
  (bind _outhit (`KismetSystemLibrary.LineTraceSingle` _returnvalue (- _returnvalue (0.0 0.0 150.0)) "TraceTypeQuery2" false (`|MakeArray` (`self.GrabbedCard`) :!type "Actor Object Reference")))
  (bind _asbpc_card_attachment (cast `/Game/Blueprints/Gameplay/Components/BPC_CardAttachment` (`.HitComponent` (`GameplayStatics.BreakHitResult` _outhit)))
    (:`then`
      (if (`/Game/Blueprints/Gameplay/Components/BPC_CardAttachment.IsEnabled` _asbpc_card_attachment)
        (if (`/Game/Blueprints/Gameplay/Components/BPC_CardAttachment.IsSlotEmpty` _asbpc_card_attachment)
          (if (== (`/Game/Blueprints/Gameplay/Card/BP_MasterCard.Team` _grabbedcard) (`/Game/Blueprints/Gameplay/Components/BPC_CardAttachment.Team` _asbpc_card_attachment))
            (if (`/Game/Blueprints/Gameplay/Components/BPC_CardAttachment.IsCardCompatible` _asbpc_card_attachment _grabbedcard)
              (return true _asbpc_card_attachment)
              (else
                _)))))
      (return false null))
    (:`CastFailed`
      (return false null))))

(fn `SendCardLocation`
  (bind _grabbedcard (`self.GrabbedCard`))
  (`self.ServerUpdateCardLocation` _grabbedcard (`Actor.K2_GetActorLocation` _grabbedcard)))

(fn `ToggleCardHighlight`
  (params (Card :type "/Game/Blueprints/Gameplay/Card/BP_MasterCard Object Reference") (IsHighlight :type Boolean))
  (`/Game/Blueprints/Gameplay/Components/BPC_Highlight.ToggleHighlight` (`/Game/Blueprints/Gameplay/Card/BP_MasterCard.BPC_Highlight` Card) IsHighlight))

(fn `ToggleInput`
  (params (Enable :type Boolean))
  (set `self.IsInputEnabled` Enable))

(fn `ToggleInteract`
  (params (StartInteraction :type Boolean))
  (if (`self.IsInputEnabled`)
    (if StartInteraction
      (bind _hoveredcard (`self.HoveredCard`)
        (:`then`
          (if (or (`/Game/Blueprints/Gameplay/Card/BP_MasterCard.IsCardDefeated` _hoveredcard) (and (`/Game/Blueprints/Gameplay/Card/BP_MasterCard.IsParalyzed` _hoveredcard) (== (`/Game/Blueprints/Gameplay/Card/BP_MasterCard.Team` _hoveredcard) (`/Game/Blueprints/Gameplay/GameMode/PS_Gameplay.Team` (`self.OwnerPS`)))))
            _
            (elif (`self.CanGrabCard` _hoveredcard)
              (bind _output_get (set `self.GrabbedCard` _hoveredcard))
              (`self.ServerToggleInteract` _output_get true (`Actor.K2_GetActorLocation` _output_get))
              (set `self.IsGrabbingCard` true)
              (bind _returnvalue (`KismetSystemLibrary.K2_SetTimerDelegate` (`|CreateDelegate` :!event `SendCardLocation`) (`self.ReplicateMovementRate`) true))
              (set `self.MovementTimer` _returnvalue)
              (`self.OnGrabToggled` true (`self.GrabbedCard`))
              (else
                (`self.ServerCardClick` _hoveredcard)))))
        (:`else`))
      (else
        (bind _grabbedcard (`self.GrabbedCard`)
          (:`then`
            (bind (_success _attachmentcomp) (`self.IsAttachmentBelow`))
            (if _success
              (`self.HandleCardSpecificConditions` _grabbedcard
                (:`Success`
                  (bind _returnvalue_2 (`Actor.K2_GetActorLocation` _grabbedcard))
                  (`self.ServerAttachCard` _grabbedcard _attachmentcomp _returnvalue_2))
                (:`Failure`
                  (`self.ServerToggleInteract` _grabbedcard false _returnvalue_2 (`/Game/Blueprints/Gameplay/Card/BP_MasterCard.GetReleaseTargetLocation` _grabbedcard) :!label _label)))
              (else
                (goto _label)))
            (set `self.IsGrabbingCard` false)
            (`KismetSystemLibrary.K2_ClearAndInvalidateTimerHandle` (`self.MovementTimer`))
            (set `self.GrabbedCard` null)
            (`self.OnGrabToggled` false))
          (:`else`))))))