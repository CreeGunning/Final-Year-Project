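; Card slot component that holds an attached card and highlights itself when empty and the player grabs a card of matching class and team.
; It listens to the local BPC_CardInteraction's grab toggle and fades a pulse material's opacity on Tick, disabling tick at the target.
; Attaching can lock grabbing; a server grab of the attached card detaches it and multicasts to restore the highlight if a grab is active.
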(event `self.ReceiveBeginPlay`
  (`/Engine/EditorBlueprintResources/StandardMacros.Can Execute Cosmetic Events`
    (:`True`
      (add `/Game/Blueprints/Gameplay/Components/BPC_CardInteraction.OnGrabToggled` (`Actor.GetComponentByClass` (`GameplayStatics.GetPlayerController` 0) "/Game/Blueprints/Gameplay/Components/BPC_CardInteraction.BPC_CardInteraction_C") (`|CreateDelegate` :!event `OnGrabToggled`))
      (bind _returnvalue (`self.CreateDynamicMaterialInstance` 0 "/Game/MaterialFunctionCollection/Materials/Materials/Pulse/MI_Pulse_03.MI_Pulse_03"))
      (set `self.Material` _returnvalue))))

(event `MulticastAttachedCardDetached`
  (if (`self.WasGrabbedToggled`)
    (`self.ToggleOpacity` true)))

(event `ToggleOpacity`
  (params (Show :type Boolean))
  (set `self.ShowOpacity` Show)
  (`self.SetComponentTickEnabled` true))

(event `self.ReceiveTick`
  (params (DeltaSeconds :type "Float (single-precision)"))
  (bind _targetopacity (`self.GetTargetOpacity`))
  (bind _material (`self.Material`))
  (bind _returnvalue (`MaterialInstanceDynamic.K2_GetScalarParameterValue` _material "Opacity"))
  (if (!= _returnvalue _targetopacity)
    (`MaterialInstanceDynamic.SetScalarParameterValue` _material "Opacity" (`KismetMathLibrary.FInterpTo_Constant` _returnvalue _targetopacity (`GameplayStatics.GetWorldDeltaSeconds`) 2.5))
    (else
      (`self.SetComponentTickEnabled` false))))

(fn `AttachCard`
  (params (Card :type "/Game/Blueprints/Gameplay/Card/BP_MasterCard Object Reference"))
  (bind _output_get (set `self.AttachedCard` Card))
  (add `/Game/Blueprints/Gameplay/Card/BP_MasterCard.ServerGrabbed` _output_get (`|CreateDelegate` :!event `OnAttachedCardGrabbed`))
  (`self.Attached`)
  (if (`self.DisableGrabOnAttach`)
    (set `/Game/Blueprints/Gameplay/Card/BP_MasterCard.CanGrab` false (`self.AttachedCard`))))

(fn `DetachCard`
  (remove `/Game/Blueprints/Gameplay/Card/BP_MasterCard.ServerGrabbed` (`self.AttachedCard`) (`|CreateDelegate` :!event `OnAttachedCardGrabbed`))
  (`self.Detached`)
  (set `self.AttachedCard` null))

(fn `GetTargetOpacity`
  (returns (TargetOpacity :type "Float (double-precision)"))
  (return (select `bool` (`self.ShowOpacity`) :`true` 1.0)))

(fn `IsCardCompatible`
  (params (Card :type "/Game/Blueprints/Gameplay/Card/BP_MasterCard Object Reference"))
  (returns (Success :type Boolean))
  (bind _returnvalue (`GameplayStatics.GetObjectClass` Card))
  (bind _cardclass (`self.CardClass`))
  (return (or (== _returnvalue _cardclass) (`KismetMathLibrary.ClassIsChildOf` _returnvalue _cardclass))))

(fn `IsSlotEmpty`
  (returns (Success :type Boolean))
  (return (not (`KismetSystemLibrary.IsValid` (`self.AttachedCard`)))))

(fn `OnAttachedCardGrabbed`
  (params (Card :type "/Game/Blueprints/Gameplay/Card/BP_MasterCard Object Reference"))
  (`self.DetachCard`)
  (`self.MulticastAttachedCardDetached`))

(fn `OnGrabToggled`
  (params (IsGrabbed :type Boolean) (Card :type "/Game/Blueprints/Gameplay/Card/BP_MasterCard Object Reference"))
  (if (`self.IsEnabled`)
    (if IsGrabbed
      (if (`self.IsCardCompatible` Card)
        (if (== (`/Game/Blueprints/Gameplay/Card/BP_MasterCard.Team` Card) (`self.Team`))
          (set `self.WasGrabbedToggled` IsGrabbed :!label _label)
          (if (`self.IsSlotEmpty`)
            (`self.ToggleOpacity` IsGrabbed))))
      (else
        (goto _label)))))