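; Card attack area actor that animates a set of cards flying into its own location as an attack.
; A server event forwards the cards to a multicast, which caches their starting locations.
; A timeline lerps each card from its cached location to the area, spawns an explosion emitter on its Smoke event track, and calls the AttackComplete dispatcher when finished.
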(event `ServerCardsAttack`
  (params (Cards :type "Array of /Game/Blueprints/Gameplay/Card/BP_MasterCard Object Reference"))
  (`self.MulticastCardsAttack` Cards))

(event `MulticastCardsAttack`
  (params (Cards :type "Array of /Game/Blueprints/Gameplay/Card/BP_MasterCard Object Reference"))
  (bind _locations (`self.CacheCardLocations` Cards))
  (set `self.CardLocations` _locations)
  (bind (_direction _alpha) (`Timeline|AttackTimeline` :!via `PlayFromStart`)
    (:`Update`
      (for (_array_element _array_index) Cards
        (`self.K2_SetActorLocation` _array_element (`KismetMathLibrary.VLerp` (`|GetArrayItem` (`self.CardLocations`) _array_index) (`self.K2_GetActorLocation`) _alpha) false false)))
    (:`Finished`
      (`self.AttackComplete`))
    (:`Smoke`
      (`GameplayStatics.SpawnEmitterAtLocation` "/Game/StarterContent/Particles/P_Explosion.P_Explosion" (`self.K2_GetActorLocation`)))))

(fn `CacheCardLocations`
  (params (Cards :type "Array of /Game/Blueprints/Gameplay/Card/BP_MasterCard Object Reference"))
  (returns (Locations :type "Array of Vector Structure"))
  (locals (LocationsTemp :type "Array of Vector Structure"))
  (for _array_element Cards
    (`KismetArrayLibrary.Array_Add` (`local.LocationsTemp`) (`self.K2_GetActorLocation` _array_element)))
  (return (`local.LocationsTemp`)))

(fn `UserConstructionScript`)