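; Networked base actor for a game card, handling grabbing, moving, releasing, attaching, flipping, selection and status display.
; Server events fire multicasts that drive timelines for transforms, with non-instigating clients interpolating toward the dragged location.
; Released cards can auto-return to their origin, while entity cards flip after attaching to a card attachment.
; RepNotifies show selection lift, fire on defeat and paralysis text.
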(event `MulticastRotate`
  (params (InitRotation :type "Rotator Structure") (TargetRotation :type "Rotator Structure"))
  (bind (_direction _alpha) (`Timeline|RotateTimeline` :!via `PlayFromStart`)
    (:`Update`
      (`self.K2_SetActorRotation` (`KismetMathLibrary.RLerp` InitRotation TargetRotation _alpha true)))))

(event `MulticastScale`
  (params (InitScale :type "Vector Structure") (TargetScale :type "Vector Structure"))
  (bind (_direction _alpha) (`Timeline|ScaleTimeline` :!via `PlayFromStart`)
    (:`Update`
      (`self.SetActorScale3D` (`KismetMathLibrary.VLerp` InitScale TargetScale _alpha)))))

(event `self.ReceiveBeginPlay`
  (`/Engine/EditorBlueprintResources/ActorMacros.Switch Has Authority`
    (:`Authority`
      (set `self.OriginLocation` (`self.K2_GetActorLocation`))
      (set `self.OriginRotation` (`self.K2_GetActorRotation`)))))

(event `ServerToggleMovement`
  (params (IsMoving :type Boolean) (InitLocation :type "Vector Structure") (InstigatorPS :type "/Game/Blueprints/Gameplay/GameMode/PS_Gameplay Object Reference"))
  (`self.MulticastToggleMovement` IsMoving InitLocation InstigatorPS)
  (if IsMoving
    (`self.ServerGrabbed` self)
    (else
      (`self.ServerReleased` self))))

(event `MulticastToggleMovement`
  (params (IsMoving :type Boolean) (InitLocation :type "Vector Structure") (InstigatorPS :type "/Game/Blueprints/Gameplay/GameMode/PS_Gameplay Object Reference"))
  (set `self.CurrentMovementLocation` InitLocation)
  (set `self.Instigator PS` InstigatorPS)
  (set `self.Is Moving` IsMoving))

(event `self.ReceiveTick`
  (params (DeltaSeconds :type "Float (single-precision)"))
  (if (`self.Is Moving`)
    (if (!= (`self.Instigator PS`) (`Controller.PlayerState` (`GameplayStatics.GetPlayerController` 0)))
      (`self.K2_SetActorLocation` (`KismetMathLibrary.VInterpTo` (`self.K2_GetActorLocation`) (`self.CurrentMovementLocation`) (`GameplayStatics.GetWorldDeltaSeconds`) 7.5)))))

(event `ServerReleaseCard`
  (params (InitLocation :type "Vector Structure") (TargetLocation :type "Vector Structure"))
  (`self.MulticastReleaseCard` InitLocation (select `bool` (`self.AutoReturn`) :`false` TargetLocation :`true` (`self.OriginLocation`))))

(event `MulticastReleaseCard`
  (params (InitLocation :type "Vector Structure") (TargetLocation :type "Vector Structure"))
  (set `self.Is Moving` false)
  (set `self.InitLocation` InitLocation)
  (set `self.TargetLocation` TargetLocation)
  (`self.K2_SetActorLocation` (`self.InitLocation`))
  (bind (_direction _alpha) (`Timeline|CardReleaseTimeline` :!via `PlayFromStart` :!label _label)
    (:`Update`
      (`self.K2_SetActorLocation` (`KismetMathLibrary.VLerp` (`self.InitLocation`) (`self.TargetLocation`) _alpha)))))

(event `MulticastOnGrabbed`
  (`|ExecutionSequence`
    (:`then_0`
      (goto _label :!via `Stop`))
    (:`then_1`
      (bind (_direction _alpha) (`Timeline|AttachCardTimeline` :!via `Stop` :!label _label_2)
        (:`Update`
          (`self.K2_SetActorRotation` (`KismetMathLibrary.ComposeRotators` (`SceneComponent.K2_GetComponentRotation` (stale `MulticastAttachCard` CardAttachment)) (struct :`Pitch` 180.0)))
          (`self.K2_SetActorLocation` (`KismetMathLibrary.VLerp` (`self.InitLocation`) (`SceneComponent.K2_GetComponentLocation` (stale `MulticastAttachCard` CardAttachment)) _alpha)))
        (:`Finished`
          (switch `ETimelineDirection` _direction
            (:`Forward`
              (`/Engine/EditorBlueprintResources/ActorMacros.Switch Has Authority`
                (:`Authority`
                  (if (`KismetMathLibrary.ClassIsChildOf` (`GameplayStatics.GetObjectClass` self) "/Game/Blueprints/Gameplay/Card/BP_MasterEntityCard.BP_MasterEntityCard_C")
                    (`self.ServerFlipCard`)))))))))))

(event `ServerOnGrabbed`
  (`self.MulticastOnGrabbed`))

(event `ServerAttachCard`
  (params (CardAttachment :type "/Game/Blueprints/Gameplay/Components/BPC_CardAttachment Object Reference") (InitLocation :type "Vector Structure"))
  (`self.ServerAttached` self)
  (`self.MulticastAttachCard` CardAttachment InitLocation)
  (`/Game/Blueprints/Gameplay/Components/BPC_CardAttachment.AttachCard` CardAttachment self))

(event `MulticastAttachCard`
  (params (CardAttachment :type "/Game/Blueprints/Gameplay/Components/BPC_CardAttachment Object Reference") (InitLocation :type "Vector Structure"))
  (set `self.InitLocation` InitLocation)
  (`self.K2_SetActorLocation` (`self.InitLocation`))
  (goto _label_2 :!via `PlayFromStart`))

(event `MulticastSpawnEffect`
  (params (ParticleSystem :type "ParticleSystem Object Reference"))
  (`/Engine/EditorBlueprintResources/StandardMacros.Can Execute Cosmetic Events`
    (:`True`
      (`GameplayStatics.SpawnEmitterAtLocation` ParticleSystem (`self.K2_GetActorLocation`)))))

(event `MulticastInstantScale`
  (params (NewScale3D :type "Vector Structure"))
  (`self.SetActorScale3D` NewScale3D))

(event `ServerFlipCard`
  (`self.MulticastFlipCard`))

(event `MulticastFlipCard`
  (bind _initrotation (`self.InitRotation`))
  (bind _initlocation (`self.InitLocation`))
  (set `self.InitRotation` (`self.K2_GetActorRotation`))
  (set `self.InitLocation` (`self.K2_GetActorLocation`))
  (bind (_direction _zalpha _rotationalpha) (`Timeline|FlipCardTimeline` :!via `PlayFromStart`)
    (:`Update`
      (`self.K2_SetActorRotation` (`KismetMathLibrary.RLerp` _initrotation (`KismetMathLibrary.ComposeRotators` _initrotation (struct :`Pitch` 180.0)) _rotationalpha true))
      (`self.K2_SetActorLocation` (`KismetMathLibrary.VLerp` _initlocation (+ _initlocation (0.0 0.0 50.0)) _zalpha)))))

(event `ServerSelectCard`
  (params (IsCardSelected :type Boolean))
  (set `self.IsCardSelected` IsCardSelected))

(event `UpdateCardSelected`
  (bind _preselectlocation (`self.PreselectLocation`))
  (if (`self.IsCardSelected`)
    (`|ExecutionSequence`
      (:`then_0`
        (`/Engine/EditorBlueprintResources/StandardMacros.DoOnce` false
          (:`Completed`
            (`/Engine/EditorBlueprintResources/ActorMacros.Switch Has Authority`
              (:`Authority`
                (set `self.PreselectLocation` (`self.K2_GetActorLocation`)))))))
      (:`then_1`
        (bind (_direction _alpha) (`Timeline|SelectTimeline` :!label _label_3)
          (:`Update`
            (`self.K2_SetActorLocation` (`KismetMathLibrary.VLerp` _preselectlocation (+ _preselectlocation (0.0 0.0 30.0)) _alpha))))))
    (else
      (goto _label_3 :!via `Reverse`))))

(event `Defeated`
  (set `self.IsCardDefeated` true)
  (`self.ServerDefeated` self))

(fn `GetActorsOfClass`
  (params (ActorClass :type "Actor Class Reference"))
  (returns (OutActors :type "Array of Actor Object Reference"))
  (bind _outactors (`GameplayStatics.GetAllActorsOfClass` ActorClass))
  (return _outactors))

(fn `GetReleaseTargetLocation`
  (returns (Location :type "Vector Structure"))
  (bind _returnvalue (`self.K2_GetActorLocation`))
  (bind _outhit (`KismetSystemLibrary.LineTraceSingle` _returnvalue (- _returnvalue (0.0 0.0 150.0)) "TraceTypeQuery1"))
  (return (`KismetMathLibrary.SelectVector` (`.Location` (`GameplayStatics.BreakHitResult` _outhit)) (`.TraceEnd` (`GameplayStatics.BreakHitResult` _outhit)) (`GameplayStatics.BreakHitResult` _outhit))))

(fn `IsParalyzed`
  (returns (Success :type Boolean))
  (return (> (`self.ParalyzedState`) 0)))

(fn `OnRep_IsCardDefeated`
  (if (`self.IsCardDefeated`)
    (bind _returnvalue (`GameplayStatics.SpawnEmitterAttached` "/Game/StarterContent/Particles/P_Fire.P_Fire" (`self.Cube`)))
    (set `self.Fire` _returnvalue)
    (else
      (bind _fire (`self.Fire`)
        (:`then`
          (`ActorComponent.K2_DestroyComponent` _fire))
        (:`else`
          _))
      (set `self.Fire` null))))

(fn `OnRep_IsCardSelected`
  (`self.UpdateCardSelected`))

(fn `OnRep_ParalyzedState`
  (`SceneComponent.SetVisibility` (`self.TextRender`) (> (`self.ParalyzedState`) 0) false))

(fn `UserConstructionScript`)