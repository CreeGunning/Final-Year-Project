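; Card ability that raises the Attack of friendly cards on the board when executed.
; It scans every card slot actor and matches the attachment component's team to the owner card's team.
; Each valid attached card that casts to a master entity card gets AttackToAdd added to its Attack, with no exclusion for the owner itself.
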(event `self.OnExecuteAbility`
  (params (OwnerCard :type "/Game/Blueprints/Gameplay/Card/BP_MasterCard Object Reference") (TargetCard :type "/Game/Blueprints/Gameplay/Card/BP_MasterCard Object Reference"))
  (bind _outactors (`/Game/Blueprints/Gameplay/Card/BP_MasterCard.GetActorsOfClass` OwnerCard "/Game/Blueprints/Gameplay/Card/BP_CardSlot.BP_CardSlot_C"))
  (for _array_element _outactors
    (bind _asbp_card_slot (cast `/Game/Blueprints/Gameplay/Card/BP_CardSlot` _array_element))
    (bind _bpc_cardattachment (`/Game/Blueprints/Gameplay/Card/BP_CardSlot.BPC_CardAttachment` _asbp_card_slot))
    (if (== (`/Game/Blueprints/Gameplay/Components/BPC_CardAttachment.Team` _bpc_cardattachment) (`/Game/Blueprints/Gameplay/Card/BP_MasterCard.Team` OwnerCard))
      (bind _attachedcard (`/Game/Blueprints/Gameplay/Components/BPC_CardAttachment.AttachedCard` _bpc_cardattachment)
        (:`then`
          (bind _asbp_master_entity_card (cast `/Game/Blueprints/Gameplay/Card/BP_MasterEntityCard` _attachedcard))
          (set `/Game/Blueprints/Gameplay/Card/BP_MasterEntityCard.Attack` (+ (`/Game/Blueprints/Gameplay/Card/BP_MasterEntityCard.Attack` _asbp_master_entity_card) (`self.AttackToAdd`)) _asbp_master_entity_card))
        (:`else`)))))