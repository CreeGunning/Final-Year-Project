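; Scene component holding a player's card hand, with server-side card spawning and a replicated Cards array.
; Tick eases idle cards into a centered row, fanned and oriented from the camera.
; Server card events scale and rotate cards on grab or release and drop attached ones from the hand.
; After retrying until controller and PlayerState exist, it tracks team on the server and toggles placeability on the owning client by turn and spirit cost.
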(event `OnClientUpdatedTurn`
  (params (IsTurn :type Boolean))
  (set `self.Is Turn` IsTurn)
  (bind _ownerps (`self.OwnerPS`)
    (:`then`
      (`self.OnUpdatedSpirit` (`/Game/Blueprints/Gameplay/GameMode/PS_Gameplay.CurrentSpirit` _ownerps)))
    (:`else`)))

(event `InitOwningClient`
  (bind _aspawn (cast `Pawn` (`self.GetOwner`)))
  (bind _aspc_gameplay (cast `/Game/Blueprints/Gameplay/GameMode/PC_Gameplay` (`Pawn.GetController` _aspawn) :!label _label)
    (:`then`
      (bind _playerstate (`/Game/Blueprints/Gameplay/GameMode/PC_Gameplay.GetPlayerState` _aspc_gameplay))
      (`/Engine/EditorBlueprintResources/StandardMacros.IsValid` _playerstate :!label _label_2
        (:`Is Valid`
          (add `/Game/Blueprints/Gameplay/GameMode/PS_Gameplay.UpdatedSpirit` _playerstate (delegate `OnUpdatedSpirit`))
          (`self.OnUpdatedSpirit` (`/Game/Blueprints/Gameplay/GameMode/PS_Gameplay.CurrentSpirit` _playerstate))
          (bind _output_get (set `self.OwnerPS` _playerstate))
          (add `/Game/Blueprints/Gameplay/GameMode/PS_Gameplay.UpdatedTurn` _playerstate (`|CreateDelegate` :!event `OnClientUpdatedTurn`))
          (`self.OnClientUpdatedTurn` (`/Game/Blueprints/Gameplay/GameMode/PS_Gameplay.IsTurn` _output_get)))
        (:`Is Not Valid`
          (`KismetSystemLibrary.Delay` 0.1)
          (goto _label_2))))
    (:`CastFailed`
      (`KismetSystemLibrary.Delay` 0.1)
      (goto _label))))

(event `OnUpdatedSpirit`
  (params (Spirit :type Integer))
  (for _array_element (`self.Cards`)
    (if (`self.Is Turn`)
      (bind _asbp_master_entity_card (cast `/Game/Blueprints/Gameplay/Card/BP_MasterEntityCard` _array_element)
        (:`then`
          (`/Game/Blueprints/Gameplay/Card/BP_MasterCard.ToggleCanPlace` _asbp_master_entity_card (>= Spirit (`/Game/Blueprints/Gameplay/Card/BP_MasterEntityCard.SpiritCost` _asbp_master_entity_card))))
        (:`CastFailed`
          (`/Game/Blueprints/Gameplay/Card/BP_MasterCard.ToggleCanPlace` _array_element true)))
      (else
        (`/Game/Blueprints/Gameplay/Card/BP_MasterCard.ToggleCanPlace` _array_element false)))))

(event `self.ReceiveBeginPlay`
  (`/Engine/EditorBlueprintResources/ActorComponentMacros.Switch Has Authority`
    (:`Authority`
      (bind _aspawn (cast `Pawn` (`self.GetOwner`)))
      (bind _aspc_gameplay (cast `/Game/Blueprints/Gameplay/GameMode/PC_Gameplay` (`Pawn.GetController` _aspawn) :!label _label_3)
        (:`then`
          (bind _playerstate (`/Game/Blueprints/Gameplay/GameMode/PC_Gameplay.GetPlayerState` _aspc_gameplay))
          (`/Engine/EditorBlueprintResources/StandardMacros.IsValid` _playerstate :!label _label_4
            (:`Is Valid`
              (add `/Game/Blueprints/Gameplay/GameMode/PS_Gameplay.UpdatedTeam` _playerstate (delegate `OnUpdatedTeam`))
              (set `self.OwnerTeam` (`/Game/Blueprints/Gameplay/GameMode/PS_Gameplay.Team` _playerstate)))
            (:`Is Not Valid`
              (`KismetSystemLibrary.Delay` 0.1)
              (goto _label_4))))
        (:`CastFailed`
          (`KismetSystemLibrary.Delay` 0.1)
          (goto _label_3))))))

(event `AssignCard`
  (params (Card :type "/Game/Blueprints/Gameplay/Card/BP_MasterCard Object Reference"))
  (bind (_returnvalue_location _returnvalue_rotation) (`KismetMathLibrary.BreakTransform` (`self.K2_GetComponentToWorld`)))
  (`KismetArrayLibrary.Array_Add` (`self.Cards`) Card)
  (add `/Game/Blueprints/Gameplay/Card/BP_MasterCard.ServerGrabbed` Card (`|CreateDelegate` :!event `OnServerCardGrabbed`))
  (add `/Game/Blueprints/Gameplay/Card/BP_MasterCard.ServerReleased` Card (`|CreateDelegate` :!event `OnServerCardReleased`))
  (add `/Game/Blueprints/Gameplay/Card/BP_MasterCard.ServerAttached` Card (`|CreateDelegate` :!event `OnServerCardAttached`))
  (set `/Game/Blueprints/Gameplay/Card/BP_MasterCard.OriginRotation` _returnvalue_rotation Card)
  (`/Game/Blueprints/Gameplay/Card/BP_MasterCard.MulticastInstantScale` Card (`KismetMathLibrary.Conv_DoubleToVector` (`self.ScaleMultiplier`)))
  (set `/Game/Blueprints/Gameplay/Card/BP_MasterCard.CanHover` true Card))

(event `OnUpdatedTeam`
  (params (Team :type Integer))
  (set `self.OwnerTeam` Team))

(event `ServerAddCard`
  (params (CardClass :type "/Game/Blueprints/Gameplay/Card/BP_MasterCard Class Reference"))
  (bind (_returnvalue_location _returnvalue_rotation) (`KismetMathLibrary.BreakTransform` (`self.K2_GetComponentToWorld`)))
  (bind _returnvalue (`|SpawnActorFromClass` CardClass (`KismetMathLibrary.MakeTransform` (0.0 0.0 0.0) _returnvalue_rotation (`KismetMathLibrary.Conv_DoubleToVector` (`self.ScaleMultiplier`))) "Undefined" "OverrideRootScale" null (`self.OwnerTeam`) true true null))
  (`KismetArrayLibrary.Array_Add` (`self.Cards`) _returnvalue)
  (add `/Game/Blueprints/Gameplay/Card/BP_MasterCard.ServerGrabbed` _returnvalue (`|CreateDelegate` :!event `OnServerCardGrabbed`))
  (add `/Game/Blueprints/Gameplay/Card/BP_MasterCard.ServerReleased` _returnvalue (`|CreateDelegate` :!event `OnServerCardReleased`))
  (add `/Game/Blueprints/Gameplay/Card/BP_MasterCard.ServerAttached` _returnvalue (`|CreateDelegate` :!event `OnServerCardAttached`)))

(event `ClientRemoveCanPlace`
  (params (Card :type "/Game/Blueprints/Gameplay/Card/BP_MasterCard Object Reference"))
  (`/Game/Blueprints/Gameplay/Card/BP_MasterCard.ToggleCanPlace` Card false))

(event `self.ReceiveTick`
  (params (DeltaSeconds :type "Float (single-precision)"))
  (bind _returnvalue (* (`Actor.K2_GetActorRotation` (`GameplayStatics.GetPlayerCameraManager` 0)) -1.0))
  (bind _returnvalue_2 (`KismetMathLibrary.Conv_VectorToRotator` (`KismetMathLibrary.RotateAngleAxis` (`KismetMathLibrary.GetForwardVector` _returnvalue) 90.0 (`KismetMathLibrary.GetRightVector` _returnvalue))))
  (for (_array_element _array_index) (`self.Cards`)
    (`/Engine/EditorBlueprintResources/StandardMacros.IsValid` _array_element
      (:`Is Valid`
        (if (not (`/Game/Blueprints/Gameplay/Card/BP_MasterCard.Is Moving` _array_element))
          (`Actor.K2_SetActorLocation` _array_element (`KismetMathLibrary.VInterpTo` (`Actor.K2_GetActorLocation` _array_element) (`self.GetCardTargetLocation` _array_index) (`GameplayStatics.GetWorldDeltaSeconds`) (`self.CardMoveSpeed`)) false false)
          (`Actor.K2_SetActorRotation` _array_element (`KismetMathLibrary.Conv_VectorToRotator` (`KismetMathLibrary.RotateAngleAxis` (`KismetMathLibrary.Conv_RotatorToVector` _returnvalue_2) (`KismetMathLibrary.MapRangeClamped` (`KismetMathLibrary.Conv_IntToDouble` _array_index) 0.0 (`KismetMathLibrary.Conv_IntToDouble` (`KismetArrayLibrary.Array_LastIndex` (`self.Cards`))) 10.0 -10.0) (`KismetMathLibrary.GetUpVector` _returnvalue_2))) false))))))

(fn `ClearHand`
  (locals (TempCards :type "Array of /Game/Blueprints/Gameplay/Card/BP_MasterCard Object Reference"))
  (bind _tempcards (`local.TempCards`))
  (set `local.TempCards` (`self.Cards`))
  (`KismetArrayLibrary.Array_Clear` (`self.Cards`))
  (for _array_element _tempcards
    (`/Engine/EditorBlueprintResources/StandardMacros.IsValid` _array_element
      (:`Is Valid`
        (`Actor.K2_DestroyActor` _array_element))))
  (`KismetArrayLibrary.Array_Clear` _tempcards))

(fn `GetCardTargetLocation`
  (params (CardIndex :type Integer))
  (returns (CardTargetLocation :type "Vector Structure"))
  (bind _returnvalue (`KismetArrayLibrary.Array_Length` (`self.Cards`)))
  (bind _returnvalue_2 (* (`self.CardWidth`) (`self.ScaleMultiplier`)))
  (return (+ (`self.K2_GetComponentLocation`) (* (`self.GetRightVector`) (+ (+ (* (/ (+ (* _returnvalue (* (`self.CardWidth`) (`self.ScaleMultiplier`))) (* (- _returnvalue 1) (`self.CardSpacing`))) 2.0) -1.0) (/ _returnvalue_2 2.0)) (* CardIndex (+ _returnvalue_2 (`self.CardSpacing`))))))))

(fn `OnRep_Cards`
  (bind _ownerps (`self.OwnerPS`)
    (:`then`
      (`self.OnUpdatedSpirit` (`/Game/Blueprints/Gameplay/GameMode/PS_Gameplay.CurrentSpirit` _ownerps)))
    (:`else`)))

(fn `OnServerCardAttached`
  (params (Card :type "/Game/Blueprints/Gameplay/Card/BP_MasterCard Object Reference"))
  (`KismetArrayLibrary.Array_RemoveItem` (`self.Cards`) Card)
  (remove `/Game/Blueprints/Gameplay/Card/BP_MasterCard.ServerGrabbed` Card (`|CreateDelegate` :!event `OnServerCardGrabbed`))
  (remove `/Game/Blueprints/Gameplay/Card/BP_MasterCard.ServerReleased` Card (`|CreateDelegate` :!event `OnServerCardReleased`))
  (remove `/Game/Blueprints/Gameplay/Card/BP_MasterCard.ServerAttached` Card (`|CreateDelegate` :!event `OnServerCardAttached`))
  (`self.ClientRemoveCanPlace` (`local.Card`)))

(fn `OnServerCardGrabbed`
  (params (Card :type "/Game/Blueprints/Gameplay/Card/BP_MasterCard Object Reference"))
  (set `/Game/Blueprints/Gameplay/Card/BP_MasterCard.OriginLocation` (`self.GetCardTargetLocation` (`KismetArrayLibrary.Array_Find` (`self.Cards`) Card)) Card)
  (`/Game/Blueprints/Gameplay/Card/BP_MasterCard.MulticastScale` Card (`Actor.GetActorScale3D` Card) (1.0 1.0 1.0))
  (`/Game/Blueprints/Gameplay/Card/BP_MasterCard.MulticastRotate` Card (`Actor.K2_GetActorRotation` Card) (`/Game/Blueprints/General/BFL_General.GetTeamCardRotation` (`self.OwnerTeam`))))

(fn `OnServerCardReleased`
  (params (Card :type "/Game/Blueprints/Gameplay/Card/BP_MasterCard Object Reference"))
  (`/Game/Blueprints/Gameplay/Card/BP_MasterCard.MulticastScale` Card (`Actor.GetActorScale3D` Card) (`KismetMathLibrary.Conv_DoubleToVector` (`self.ScaleMultiplier`)))
  (`/Game/Blueprints/Gameplay/Card/BP_MasterCard.MulticastRotate` Card (`Actor.K2_GetActorRotation` Card) (`self.K2_GetComponentRotation`)))