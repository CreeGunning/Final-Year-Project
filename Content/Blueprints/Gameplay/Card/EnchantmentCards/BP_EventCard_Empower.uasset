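; Empower enchantment event card that buffs the health and attack of the entity card in its target slot.
; On execution it takes the card attached to the target slot and, if it is a master entity card, adds the configured health and attack amounts.
; A successful buff also multicasts a smoke effect, and the event signals completion.
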(event `self.OnExecuteEvent`
  (params (TargetCardSlot :type "/Game/Blueprints/Gameplay/Card/BP_CardSlot Object Reference"))
  (bind _attachedcard (`/Game/Blueprints/Gameplay/Components/BPC_CardAttachment.AttachedCard` (`/Game/Blueprints/Gameplay/Card/BP_CardSlot.BPC_CardAttachment` TargetCardSlot))
    (:`then`
      (bind _asbp_master_entity_card (cast `/Game/Blueprints/Gameplay/Card/BP_MasterEntityCard` _attachedcard)
        (:`then`
          (set `/Game/Blueprints/Gameplay/Card/BP_MasterEntityCard.Health` (+ (`/Game/Blueprints/Gameplay/Card/BP_MasterEntityCard.Health` _asbp_master_entity_card) (`self.HealthToAdd`)) _asbp_master_entity_card)
          (set `/Game/Blueprints/Gameplay/Card/BP_MasterEntityCard.Attack` (+ (`/Game/Blueprints/Gameplay/Card/BP_MasterEntityCard.Attack` _asbp_master_entity_card) (`self.AttackToAdd`)) _asbp_master_entity_card)
          (`self.MulticastSpawnEffect` "/Game/StarterContent/Particles/P_Smoke1.P_Smoke1"))
        (:`CastFailed`
          _)))
    (:`else`
      _))
  (`self.EventCompleted`))

(fn `UserConstructionScript`
  (`parent.UserConstructionScript`))