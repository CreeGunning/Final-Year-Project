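; Base Blueprint for entity cards, holding Health, Attack and StaminaCost and displaying each as text on the card.
; Each stat has a RepNotify that refreshes its text, and BeginPlay sets all three, only where cosmetic events can execute.
; ApplyDamage subtracts from Health with a floor of zero, calls Defeated at zero and returns whether the card was defeated.
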(event `self.ReceiveBeginPlay`
  (`parent.ReceiveBeginPlay`)
  (`/Engine/EditorBlueprintResources/StandardMacros.Can Execute Cosmetic Events`
    (:`True`
      (`self.UpdateHealthText`)
      (`self.UpdateAttackText`)
      (`self.UpdateStaminaText`))))

(fn `ApplyDamage`
  (params (Damage :type Integer))
  (returns (Defeated :type Boolean))
  (bind _output_get (set `self.Health` (`KismetMathLibrary.Max` (- (`self.Health`) Damage))))
  (if (== _output_get 0)
    (`self.Defeated`)
    (return true)
    (else
      (return false))))

(fn `OnRep_Attack`
  (`/Engine/EditorBlueprintResources/StandardMacros.Can Execute Cosmetic Events`
    (:`True`
      (`self.UpdateAttackText`))))

(fn `OnRep_Health`
  (`/Engine/EditorBlueprintResources/StandardMacros.Can Execute Cosmetic Events`
    (:`True`
      (`self.UpdateHealthText`))))

(fn `OnRep_StaminaCost`
  (`/Engine/EditorBlueprintResources/StandardMacros.Can Execute Cosmetic Events`
    (:`True`
      (`self.UpdateStaminaText`))))

(fn `UpdateAttackText`
  (`TextRenderComponent.K2_SetText` (`self.AttackText`) (`KismetTextLibrary.Conv_IntToText` (`self.Attack`))))

(fn `UpdateHealthText`
  (`TextRenderComponent.K2_SetText` (`self.HealthText`) (`KismetTextLibrary.Conv_IntToText` (`self.Health`))))

(fn `UpdateStaminaText`
  (`TextRenderComponent.K2_SetText` (`self.StaminaText`) (`KismetTextLibrary.Conv_IntToText` (`self.StaminaCost`))))

(fn `UserConstructionScript`
  (`parent.UserConstructionScript`))