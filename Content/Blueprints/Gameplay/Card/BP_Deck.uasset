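; BP_Deck is a card deck actor that spawns and deals a team's stack of cards.
; SetupDeck stacks random unit or event cards, flipped and ungrabbable, each raised by a height offset, then places a random leader card on top.
; ReceiveCard pops the last card from the stack, makes it grabbable and returns it, while the leader card is stored separately.
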(event `SetupDeck`
  (params (TotalCards :type Integer))
  (bind (_returnvalue_x _returnvalue_y _returnvalue_z) (`KismetMathLibrary.BreakVector` (`self.K2_GetActorLocation`)))
  (bind (_returnvalue_roll _returnvalue_pitch _returnvalue_yaw) (`KismetMathLibrary.BreakRotator` (`self.K2_GetActorRotation`)))
  (bind (_returnvalue_roll_2 _returnvalue_pitch_2 _returnvalue_yaw_2) (`KismetMathLibrary.BreakRotator` (`self.K2_GetActorRotation`)))
  (bind (_returnvalue_x_2 _returnvalue_y_2 _returnvalue_z_2) (`KismetMathLibrary.BreakVector` (`self.K2_GetActorLocation`)))
  (for _index (range TotalCards)
    (bind _returnvalue (`|SpawnActorFromClass` (`self.GetRandomCard`) (`KismetMathLibrary.MakeTransform` (`KismetMathLibrary.MakeVector` _returnvalue_x_2 _returnvalue_y_2 (+ _returnvalue_z_2 (* _index (`self.CardHeightOffset`)))) (`KismetMathLibrary.MakeRotator` 0.0 180.0 _returnvalue_yaw_2)) "Undefined" "OverrideRootScale" null (`self.Team`) true false null))
    (`KismetArrayLibrary.Array_Add` (`self.Cards`) _returnvalue)
    (set `/Game/Blueprints/Gameplay/Card/BP_MasterCard.CanGrab` false _returnvalue))
  (bind _returnvalue_2 (`|SpawnActorFromClass` (`KismetArrayLibrary.Array_Random` (`self.LeaderCards`)) (`KismetMathLibrary.MakeTransform` (`KismetMathLibrary.MakeVector` _returnvalue_x _returnvalue_y (+ _returnvalue_z (* TotalCards (`self.CardHeightOffset`)))) (`KismetMathLibrary.MakeRotator` 0.0 180.0 _returnvalue_yaw)) "Undefined" "OverrideRootScale" null (`self.Team`) true true null))
  (set `self.LeaderCard` _returnvalue_2))

(fn `GetRandomCard`
  (returns (CardClass :type "/Game/Blueprints/Gameplay/Card/BP_MasterCard Class Reference"))
  (locals (TempCards :type "Array of /Game/Blueprints/Gameplay/Card/BP_MasterCard Class Reference"))
  (bind _output_get (set `local.TempCards` (`self.UnitCards`)))
  (`KismetArrayLibrary.Array_Append` _output_get (`self.EventCards`))
  (return (`KismetArrayLibrary.Array_Random` (`local.TempCards`))))

(fn `ReceiveCard`
  (returns (Card :type "/Game/Blueprints/Gameplay/Card/BP_MasterCard Object Reference"))
  (locals (TempCard :type "/Game/Blueprints/Gameplay/Card/BP_MasterCard Object Reference"))
  (bind _cards (`self.Cards`))
  (bind _tempcard (`local.TempCard`))
  (bind _output_get (set `local.TempCard` (`|GetArrayItem` _cards (`KismetArrayLibrary.Array_LastIndex` _cards))))
  (`KismetArrayLibrary.Array_RemoveItem` _cards _output_get)
  (set `/Game/Blueprints/Gameplay/Card/BP_MasterCard.CanGrab` true _tempcard)
  (return _tempcard))

(fn `UserConstructionScript`)